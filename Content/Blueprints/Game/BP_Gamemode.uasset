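; Game mode for a find-the-target crowd game that picks a random target outfit and runs a battery countdown.
; SpawnAIs scatters pre-placed AI characters over the navmesh by difficulty, dresses one as the target and destroys the surplus.
; Others matching the target get one random clothing slot set to a fixed enum value; the filtered arrays go unused.
; A looping timer lowers the player's MultiplierTimer, triggering GameOver at zero.
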(event Custom|Lose%20One%20Battery
  (bind _playerref (Variables|Default|GetPlayerRef)
    (:then
      (bind _output_get (Variables|/Game/Blueprints/Character/BP_Player.BP_Player_C|SetMultiplier_Timer _playerref (- (Variables|/Game/Blueprints/Character/BP_Player.BP_Player_C|GetMultiplier_Timer _playerref) 0.2)))
      (if (<= _output_get 0.0)
        (Utilities|Time|ClearandInvalidateTimerbyHandle (Variables|Default|GetTimerRef))
        (Default|GameOver _playerref)))
    (:else)))

(event Custom|Spawn%20AIs
  (bind _all_ai_chars (Variables|Default|GetAll_AI_Chars))
  (bind _all_ai_chars_2 (Variables|Default|GetAll_AI_Chars))
  (bind _returnvalue (Utilities|Array|LastIndex _all_ai_chars_2))
  (bind _returnvalue_2 (Utilities|Array|LastIndex _all_ai_chars))
  (bind _output (Utilities|Array|Get(acopy) _all_ai_chars_2 _returnvalue))
  (bind _returnvalue_3 (Actor|GetActorOfClass "/Script/NavigationSystem.NavigationData"))
  (bind _output_get (Variables|Default|SetNavDataRef _returnvalue_3))
  (for _index (range 0 (Utilities|Select :Index (Variables|/Game/Blueprints/Game/GI_InstanceBase.GI_InstanceBase_C|GetDifficulty (Variables|Default|GetGInstanceRef)) :Option%200 50 :Option%201 150 :Option%202 300))
    (Transformation|SetActorLocation (Utilities|Array|Get(acopy) _all_ai_chars _returnvalue_2) (.RandomLocation (AI|Navigation|GetRandomReachablePointinRadius (Math|Vector|MakeVector 0.0 0.0 0.0) 1e+04 _output_get 0)) false false)
    (if (== _index 0)
      (Default|InitCharacterTarget _output (Variables|Default|GetTarget_Color_Shirt) (Variables|Default|GetTarget_Color_Pants) (Variables|Default|GetTarget_Mask))
      (elif (Math|Boolean|ANDBoolean (Utilities|Enum|Equal(Enum) (Variables|/Game/Blueprints/AI/BP_AI_Character.BP_AI_Character_C|GetTopColor _output) (Variables|Default|GetTarget_Color_Shirt)) (Utilities|Enum|Equal(Enum) (Variables|/Game/Blueprints/AI/BP_AI_Character.BP_AI_Character_C|GetBottomColor _output) (Variables|Default|GetTarget_Color_Pants)) (Utilities|Enum|Equal(Enum) (Variables|/Game/Blueprints/AI/BP_AI_Character.BP_AI_Character_C|GetMask _output) (Variables|Default|GetTarget_Mask)))
        (CallFunction|SwitchUpONEArticleOfClothing _output)))
    (Utilities|Array|RemoveIndex (Variables|Default|GetAll_AI_Chars) _returnvalue_2))
  (for _array_element (Variables|Default|GetAll_AI_Chars)
    (Actor|DestroyActor _array_element))
  (Development|PrintString "Hello"))

(event EventBeginPlay
  (bind _array (Utilities|Array|MakeArray "NewEnumerator0" "NewEnumerator1" "NewEnumerator2" "NewEnumerator3" "NewEnumerator4" "NewEnumerator5" "NewEnumerator6"))
  (bind _outitem (Utilities|Array|Random _array))
  (bind _returnvalue (Utilities|Time|SetTimerbyEvent (delegate Custom|Lose%20One%20Battery) 3e+02 true))
  (Variables|Default|SetTimerRef _returnvalue)
  (Variables|Default|SetTarget_Color_Shirt _outitem)
  (Variables|Default|SetTarget_Color_Pants _outitem)
  (Variables|Default|SetTarget_Mask (.OutItem (Utilities|Array|Random (Utilities|Array|MakeArray "NewEnumerator0" "NewEnumerator1" "NewEnumerator2" "NewEnumerator3" "NewEnumerator4" "NewEnumerator5" "NewEnumerator6"))))
  (bind _outactors (Actor|GetAllActorsOfClass "/Game/Blueprints/AI/BP_AI_Character.BP_AI_Character_C"))
  (Variables|Default|SetAll_AI_Chars _outactors)
  (bind _asgi_instance_base (Utilities|Casting|CastToGI_InstanceBase (Game|GetGameInstance)))
  (Variables|Default|SetGInstanceRef _asgi_instance_base)
  (CallFunction|SpawnAIs))

(event EventTick
  (params (DeltaSeconds :type Float%20%28single-precision%29)))

(fn ConstructionScript)

(fn SwitchUpONEArticleOfClothing
  (params (CharToChange :type BP%20AI%20Character%20Object%20Reference))
  (switch int (Math|Random|RandomIntegerinRange 0 2)
    (:Default
      (bind _output_get (LocalVariables|SetMaskArray (Utilities|Array|MakeArray "NewEnumerator0" "NewEnumerator1" "NewEnumerator2" "NewEnumerator3" "NewEnumerator4" "NewEnumerator5" "NewEnumerator6") :!label _label))
      (Utilities|Array|RemoveItem _output_get (Variables|Default|GetTarget_Mask))
      (Default|ChangeMask CharToChange "NewEnumerator0"))
    (:0
      (bind _output_get_2 (LocalVariables|SetColorArray (Utilities|Array|MakeArray "NewEnumerator0" "NewEnumerator1" "NewEnumerator2" "NewEnumerator3" "NewEnumerator4" "NewEnumerator5" "NewEnumerator6")))
      (Utilities|Array|RemoveItem _output_get_2 (Variables|Default|GetTarget_Color_Shirt))
      (Default|ChangeShirt CharToChange "NewEnumerator0"))
    (:1
      (bind _output_get_3 (LocalVariables|SetColorArray (Utilities|Array|MakeArray "NewEnumerator0" "NewEnumerator1" "NewEnumerator2" "NewEnumerator3" "NewEnumerator4" "NewEnumerator5" "NewEnumerator6")))
      (Utilities|Array|RemoveItem _output_get_3 (Variables|Default|GetTarget_Color_Pants))
      (Default|ChangePants CharToChange "NewEnumerator0"))
    (:2
      (goto _label))))