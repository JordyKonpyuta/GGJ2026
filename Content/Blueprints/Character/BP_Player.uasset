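; BP_Player is the player character of a photography game where one shot of a masked target ends the round, and landing counts as death.
; It handles movement, zoom-scaled look sensitivity, smoothed FOV zoom, and HUD, pause and end-game widgets.
; TakePicture triggers a scene capture, finds on-screen AI by screen projection, requires an unmasked target, then scores facing angle, crowd count, head-trace obstruction and a timer multiplier.
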(event Custom|Game%20Over
  (bind _returnvalue (UserInterface|CreateWidget "/Game/Blueprints/Widgets/WBP_EndGame.WBP_EndGame_C"))
  (Default|DisplayDeath _returnvalue)
  (UserInterface|Viewport|AddtoViewport _returnvalue 0)
  (Input|SetInputModeUIOnly (Game|GetPlayerController 0) _returnvalue "DoNotLock" true)
  (bind _asbp_gamemode (Utilities|Casting|CastToBP_Gamemode (Game|GetGameMode)))
  (Default|DeathState _asbp_gamemode))

(event Custom|Game%20Finished
  (bind _returnvalue (UserInterface|CreateWidget "/Game/Blueprints/Widgets/WBP_EndGame.WBP_EndGame_C"))
  (UserInterface|Viewport|AddtoViewport _returnvalue 0)
  (Input|SetInputModeUIOnly (Game|GetPlayerController 0) _returnvalue "DoNotLock" true)
  (Default|DisplayScore _returnvalue)
  (bind _asbp_gamemode (Utilities|Casting|CastToBP_Gamemode (Game|GetGameMode)))
  (Default|DeathState _asbp_gamemode))

(event Input|EnhancedActionEvents|EnhancedInputActionIA_Target
  (params (ActionValue :type Boolean) (ElapsedSeconds :type Float%20%28double-precision%29) (TriggeredSeconds :type Float%20%28double-precision%29) (InputAction :type Input%20Action%20Object%20Reference :default "/Game/Blueprints/Character/Mapping/InputActions/IA_Target.IA_Target"))
  (:Started
    (Default|ActionBlocNote (Variables|Refs|GetHUD_Ref))))

(event Input|EnhancedActionEvents|EnhancedInputActionIA_Pause
  (params (ActionValue :type Boolean) (ElapsedSeconds :type Float%20%28double-precision%29) (TriggeredSeconds :type Float%20%28double-precision%29) (InputAction :type Input%20Action%20Object%20Reference :default "/Game/Blueprints/Character/Mapping/InputActions/IA_Pause.IA_Pause"))
  (bind _pauseref (Variables|Default|GetPauseRef))
  (:Completed
    (UserInterface|Viewport|AddtoViewport _pauseref 0)
    (Default|StartPause _pauseref)))

(event Input|EnhancedActionEvents|EnhancedInputActionIA_Look
  (params (ActionValue :type Vector%202D%20Structure) (ElapsedSeconds :type Float%20%28double-precision%29) (TriggeredSeconds :type Float%20%28double-precision%29) (InputAction :type Input%20Action%20Object%20Reference :default "/Game/Blueprints/Character/Mapping/InputActions/IA_Look.IA_Look"))
  (bind _currentzoompercent (Variables|Camera|GetCurrentZoomPercent))
  (bind _returnvalue (* _currentzoompercent _currentzoompercent))
  (bind _returnvalue_2 (Math|Float|Lerp 1.0 5e+01 _returnvalue))
  (Pawn|Input|AddControllerYawInput (/ (* (+ 1.0 (Variables|Camera|GetSensiSouris)) (.x ActionValue)) _returnvalue_2))
  (Pawn|Input|AddControllerPitchInput (/ (* (.y ActionValue) (+ 1.0 (Variables|Camera|GetSensiSouris))) _returnvalue_2)))

(event Input|EnhancedActionEvents|EnhancedInputActionIA_TakePicture
  (params (ActionValue :type Boolean) (ElapsedSeconds :type Float%20%28double-precision%29) (TriggeredSeconds :type Float%20%28double-precision%29) (InputAction :type Input%20Action%20Object%20Reference :default "/Game/Blueprints/Character/Mapping/InputActions/IA_TakePicture.IA_TakePicture"))
  (CallFunction|TakePicture)
  (CallFunction|GameFinished))

(event Input|EnhancedActionEvents|EnhancedInputActionIA_Zoom
  (params (ActionValue :type Float%20%28double-precision%29) (ElapsedSeconds :type Float%20%28double-precision%29) (TriggeredSeconds :type Float%20%28double-precision%29) (InputAction :type Input%20Action%20Object%20Reference :default "/Game/Blueprints/Character/Mapping/InputActions/IA_Zoom.IA_Zoom"))
  (CallFunction|Zoom (>= ActionValue 0.0))
  (Variables|Camera|SetCurrentFOV (Math|Float|Lerp 9e+01 (Variables|Camera|GetMinimumFOV) (Variables|Camera|GetCurrentZoomPercent)))
  (Default|SetZoomText (Variables|Refs|GetHUD_Ref) (Math|Float|Lerp 1.0 11.0 (Variables|Camera|GetCurrentZoomPercent))))

(event Input|EnhancedActionEvents|EnhancedInputActionIA_Move
  (params (ActionValue :type Vector%202D%20Structure) (ElapsedSeconds :type Float%20%28double-precision%29) (TriggeredSeconds :type Float%20%28double-precision%29) (InputAction :type Input%20Action%20Object%20Reference :default "/Game/Blueprints/Character/Mapping/InputActions/IA_Move.IA_Move"))
  (Pawn|Input|AddMovementInput (Transformation|GetActorRightVector) (.x ActionValue) false)
  (Pawn|Input|AddMovementInput (Transformation|GetActorForwardVector) (.y ActionValue) false))

(event EventBeginPlay
  (Components|Activation|Deactivate (Variables|Default|GetSceneCaptureComponent2D))
  (bind _returnvalue (UserInterface|CreateWidget "/Game/Blueprints/Widgets/WBP_HUD.WBP_HUD_C"))
  (bind _output_get (Variables|Refs|SetHUD_Ref _returnvalue))
  (UserInterface|Viewport|AddtoViewport _output_get 0)
  (bind _asbp_gamemode (Utilities|Casting|CastToBP_Gamemode (Game|GetGameMode)))
  (Variables|/Game/Blueprints/Game/BP_Gamemode.BP_Gamemode_C|SetPlayerRef _asbp_gamemode self)
  (Default|DisplayInformations _asbp_gamemode)
  (bind _asgi_instance_base (Utilities|Casting|CastToGI_InstanceBase (Game|GetGameInstance)))
  (Variables|Camera|SetSensiSouris (Variables|/Game/Blueprints/Game/GI_InstanceBase.GI_InstanceBase_C|GetSensiSouris _asgi_instance_base))
  (bind _returnvalue_2 (UserInterface|CreateWidget "/Game/Blueprints/Widgets/WBP_Pause.WBP_Pause_C"))
  (bind _output_get_2 (Variables|Default|SetPauseRef _returnvalue_2))
  (UserInterface|Viewport|AddtoViewport _output_get_2 0)
  (Default|StopPause _returnvalue_2))

(event EventControllerChanged
  (params (OldController :type Controller%20Object%20Reference) (NewController :type Controller%20Object%20Reference))
  (bind _asbp_player_controller (Utilities|Casting|CastToBP_PlayerController NewController))
  (Input|AddMappingContext (PlayerController|LocalPlayerSubsystems|GetEnhancedInputLocalPlayerSubsystem _asbp_player_controller) "/Game/Blueprints/Character/Mapping/IMP_PlayerControls.IMP_PlayerControls" 0 "(bIgnoreAllPressedKeysUntilRelease=True,bForceImmediately=False,bNotifyUserSettings=False)"))

(event EventTick
  (params (DeltaSeconds :type Float%20%28single-precision%29))
  (bind _camera (Variables|Default|GetCamera))
  (bind _currentfov (Variables|Camera|GetCurrentFOV))
  (bind _fieldofview (Variables|/Script/Engine.CameraComponent|GetFieldOfView _camera))
  (bind _returnvalue (Math|Interpolation|FInterpTo _fieldofview _currentfov DeltaSeconds 5.0))
  (Camera|SetFieldOfView _camera _returnvalue)
  (Variables|/Script/Engine.SceneCaptureComponent2D|SetFOVAngle (Variables|Default|GetSceneCaptureComponent2D) _returnvalue))

(event Collision|EventActorBeginOverlap
  (params (OtherActor :type Actor%20Object%20Reference)))

(event EventOnLanded
  (params (Hit :type Hit%20Result%20Structure%20%28by%20ref%29))
  (CallFunction|GameOver))

(fn ConstructionScript)

(fn Zoom
  (params (GoingForward :type Boolean))
  (Variables|Camera|SetCurrentZoomPercent (Math|Float|SelectFloat (Math|Float|SelectFloat 1.0 (+ (Math|Float|SelectFloat 0.05 -0.05 GoingForward) (Variables|Camera|GetCurrentZoomPercent)) (> (+ (Math|Float|SelectFloat 0.05 -0.05 GoingForward) (Variables|Camera|GetCurrentZoomPercent)) 1.0)) (Math|Float|SelectFloat 0.0 (+ (Math|Float|SelectFloat 0.05 -0.05 GoingForward) (Variables|Camera|GetCurrentZoomPercent)) (< (+ (Math|Float|SelectFloat 0.05 -0.05 GoingForward) (Variables|Camera|GetCurrentZoomPercent)) 0.0)) GoingForward)))

(fn TakePicture
  (bind _angle (CallFunction|GetAnglewithTarget))
  (bind _scenecapturecomponent2d (Variables|Default|GetSceneCaptureComponent2D))
  (bind _returnvalue (Math|Float|Lerp 0.1 0.9 _angle))
  (Components|Activation|Activate _scenecapturecomponent2d false)
  (Rendering|SceneCapture|CaptureScene _scenecapturecomponent2d :!class /Script/Engine.SceneCaptureComponent2D)
  (Components|Activation|Deactivate _scenecapturecomponent2d)
  (Utilities|Array|Clear (Variables|Picture|GetAllActorsToLookFor))
  (Utilities|FlowControl|Sequence
    (:then_0
      (bind _outactors (Actor|GetAllActorsOfClass "/Game/Blueprints/AI/BP_AI_Character.BP_AI_Character_C"))
      (for _array_element _outactors
        (if (CallFunction|IsonPicture _array_element)
          (if (Variables|/Game/Blueprints/AI/BP_AI_Character.BP_AI_Character_C|GetIsTarget _array_element)
            (Variables|Scoring|SetMultiplier_IsOnPicture 1.0)
            (if (Variables|/Game/Blueprints/AI/BP_AI_Character.BP_AI_Character_C|GetRemovedMask _array_element)
              (Variables|Scoring|SetMultiplier_MaskRemoved 1.0)
              (Variables|Picture|SetPictureTechnicallyCorrect true)
              (Variables|Refs|SetTargetRef _array_element)
              (else
                (Variables|Scoring|SetMultiplier_MaskRemoved 0.0)))
            (else
              (Math|Integer|IncrementInt (Variables|Picture|GetNumberPeopleOnPicture))))))
      (if (Variables|Picture|GetPictureTechnicallyCorrect)
        (Variables|Scoring|SetScore 1e+02)
        (bind _output_get (Variables|Scoring|SetMultiplier_Angle (Math|Float|SelectFloat 0.0 (Math|Float|SelectFloat 1.0 _returnvalue (> _returnvalue 1.0)) (< _returnvalue 0.0))))
        (if (== _output_get 0.0)
          (return true)
          (else
            (Variables|Scoring|SetMultiplier_People (Math|Float|Clamp(Float) (- 1.0 (* (- (Variables|Picture|GetNumberPeopleOnPicture) (Variables|Default|GetLimitOfRandomPeopleAllowedOnPhoto)) 0.05)) 0.2))
            (bind _outhit (Collision|LineTraceByChannel (Transformation|GetWorldLocation (Variables|Default|GetCamera)) (.Location (Math|Transform|BreakTransform (Transformation|GetBoneTransform (Variables|/Script/Engine.Character|GetMesh (Variables|Refs|GetTargetRef)) "Head" "RTS_World"))) "TraceTypeQuery2" false 0 "Persistent"))
            (if (== (Variables|Refs|GetTargetRef) (.HitActor (Collision|BreakHitResult _outhit)))
              (Variables|Scoring|SetMultiplier_Obstacle 1.0)
              (else
                (Variables|Scoring|SetMultiplier_Obstacle 0.5)))
            (Variables|Scoring|SetScore (* 1e+02 (Variables|Scoring|GetMultiplier_Obstacle) (Variables|Scoring|GetMultiplier_Timer) (Variables|Scoring|GetMultiplier_Angle) (Variables|Scoring|GetMultiplier_People)))))
        (else
          (Variables|Scoring|SetScore 0.0)
          (return true))))
    (:then_1
      (bind _returnvalue_2 (UserInterface|CreateWidget "/Game/Blueprints/Widgets/WBP_EndGame.WBP_EndGame_C"))
      (UserInterface|Viewport|AddtoViewport _returnvalue_2 0)
      (Input|SetInputModeUIOnly (Game|GetPlayerController 0) _returnvalue_2 "DoNotLock" true)
      (Default|DisplayScore _returnvalue_2))))

(fn IsonPicture
  (params (Target :type Actor%20Object%20Reference))
  (bind _returnvalue (Game|GetPlayerController 0))
  (bind _returnvalue_2 (Transformation|GetActorLocation Target))
  (bind _returnvalue_3 (Viewport|GetViewportSize))
  (bind (_x _y _z) (Math|Vector|BreakVector _returnvalue_2))
  (bind _returnvalue_4 (+ _z 8e+01))
  (bind _returnvalue_5 (Math|Vector|MakeVector _x _y _returnvalue_4))
  (bind _screenposition (Class|GameplayStatics|ProjectWorldtoScreen _returnvalue _returnvalue_5 false))
  (return (Math|Boolean|ANDBoolean (> (.x _screenposition) 0.0) (< (.x _screenposition) (.x _returnvalue_3)) (> (.y _screenposition) 0.0) (< (.y _screenposition) (.y _returnvalue_3)))))

(fn GetAnglewithTarget
  (bind _returnvalue (Transformation|GetActorForwardVector))
  (bind _targetref (Variables|Refs|GetTargetRef))
  (bind (_x _y) (Math|Vector|BreakVector _returnvalue))
  (bind _returnvalue_2 (Transformation|GetActorForwardVector _targetref))
  (bind (_x_2 _y_2) (Math|Vector|BreakVector _returnvalue_2))
  (return (+ (* (Math|Vector2D|DotProduct(2D) (Math|Vector2D|Normalize2D (Math|Vector2D|MakeVector2D _x _y)) (Math|Vector2D|Normalize2D (Math|Vector2D|MakeVector2D _x_2 _y_2))) -1.0) 0.5)))