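; Decorative fireworks actor that launches a celebratory burst in the level every few seconds for as long as it exists.
; A looping timer started at BeginPlay fires Kblam, which spawns the fireworks Niagara system at a random wide horizontal offset around the actor's location.
; Each burst also plays a non-spatialized 2D fireworks sound, so it is heard regardless of distance.
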(event Custom|Kblam
  (Niagara|SpawnSystematLocation "/Game/VFX/VFX_Fireworks.VFX_Fireworks" (+ (Transformation|GetActorLocation) (Math|Vector|MakeVector (* (- (Math|Random|RandomInteger 120) 60) 150) (* (- (Math|Random|RandomInteger 120) 60) 150) 0.0)))
  (Audio|PlaySound2D "/Game/SFX/Ambiance/SC_Fireworks.SC_Fireworks" 1.0 1.0 0.0 0 0))

(event EventBeginPlay
  (Utilities|Time|SetTimerbyEvent (delegate Custom|Kblam) 2.0 true))

(fn ConstructionScript)