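; AI character that wanders the level as a masked NPC with randomized clothing colors and mask.
; On BeginPlay, InitCharacter picks the look, applying cloth materials and a per-mask mesh transform saved in MaskTransformRef.
; AI_Movement loops random-point moves with timed pauses, during which IsRemovingMask is sometimes set briefly.
; InitCharacter_Target applies a caller-specified color and mask combination instead of a random one.
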(event Custom|AI_Movement
  (bind _returnvalue (Math|Random|RandomBool))
  (Variables|Default|SetIsWalking true)
  (AI|AIMoveTo (AI|GetAIController self) (Math|Vector|MakeVector (Math|Random|RandomFloatinRange -3.8e+03 4.15e+03) (Math|Random|RandomFloatinRange -3.9e+03 4.05e+03) 0.0) 0 -1.0 "Default" "Default" true true
    (:OnRequestFailed
      _)
    (:OnMoveFinished
      _))
  (Variables|Default|SetIsWalking false)
  (Variables|Default|SetIsRemovingMask (and _returnvalue _returnvalue))
  (Utilities|FlowControl|Delay (Math|Random|RandomFloatinRange 2.0 4.0))
  (Variables|Default|SetIsRemovingMask false)
  (Utilities|FlowControl|Delay (Math|Random|RandomFloatinRange 2.0 4.0))
  (CallFunction|AIMovement))

(event Custom|InitCharacter_Target
  (params (TopColor :type E_Color%20Enum :default "NewEnumerator0") (InputPin :type E_Color%20Enum :default "NewEnumerator0") (Mask :type E_Mask%20Enum :default "NewEnumerator0"))
  (bind _sm_mask (Variables|Default|GetSM_Mask))
  (bind _output_get (Variables|Default|SetTopColor TopColor))
  (Rendering|Material|SetMaterial (Variables|Default|GetSK_Top) 0 (Utilities|Select :Index _output_get :NewEnumerator0 "/Game/Assets/Materials/MI_Cloth_Blue.MI_Cloth_Blue" :NewEnumerator1 "/Game/Assets/Materials/MI_Cloth_Red.MI_Cloth_Red" :NewEnumerator2 "/Game/Assets/Materials/MI_Cloth_Yellow.MI_Cloth_Yellow" :NewEnumerator3 "/Game/Assets/Materials/MI_Cloth_Green.MI_Cloth_Green" :NewEnumerator4 "/Game/Assets/Materials/MI_Cloth_Purple.MI_Cloth_Purple" :NewEnumerator5 "/Game/Assets/Materials/MI_Cloth_Pink.MI_Cloth_Pink" :NewEnumerator6 "/Game/Assets/Materials/MI_Cloth_Brown.MI_Cloth_Brown"))
  (bind _output_get_2 (Variables|Default|SetBottomColor InputPin))
  (Rendering|Material|SetMaterial (Variables|Default|GetSK_Bottom) 0 (Utilities|Select :Index _output_get_2 :NewEnumerator0 "/Game/Assets/Materials/MI_Cloth_Blue.MI_Cloth_Blue" :NewEnumerator1 "/Game/Assets/Materials/MI_Cloth_Red.MI_Cloth_Red" :NewEnumerator2 "/Game/Assets/Materials/MI_Cloth_Yellow.MI_Cloth_Yellow" :NewEnumerator3 "/Game/Assets/Materials/MI_Cloth_Green.MI_Cloth_Green" :NewEnumerator4 "/Game/Assets/Materials/MI_Cloth_Purple.MI_Cloth_Purple" :NewEnumerator5 "/Game/Assets/Materials/MI_Cloth_Pink.MI_Cloth_Pink" :NewEnumerator6 "/Game/Assets/Materials/MI_Cloth_Brown.MI_Cloth_Brown"))
  (bind _output_get_3 (Variables|Default|SetMask Mask))
  (Components|StaticMesh|SetStaticMesh _sm_mask (Utilities|Select :Index _output_get_3 :NewEnumerator0 "/Game/Assets/Masks/Kitsune/7b6eb1ca7e6c_dark_fantasy__golde.7b6eb1ca7e6c_dark_fantasy__golde" :NewEnumerator1 "/Game/Assets/Masks/Blue/delft_blue_mask.delft_blue_mask" :NewEnumerator2 "/Game/Assets/Masks/Face/Mask.Mask" :NewEnumerator3 "/Game/Assets/Masks/Plague/Mask.Mask" :NewEnumerator4 "/Game/Assets/Masks/Hockey/джасан.джасан" :NewEnumerator5 "/Game/Assets/Masks/Venetian/venetian_mask_1.venetian_mask_1" :NewEnumerator6 "/Game/Assets/Masks/Wolf/wolfmask1.wolfmask1"))
  (Transformation|SetRelativeTransform _sm_mask (Utilities|Select :Index _output_get_3 :NewEnumerator0 (Math|Transform|MakeTransform "0.000000,-20.000000,15.000000" "90.000000,0.000000,-90.000000" "0.400000,0.400000,0.400000") :NewEnumerator1 (Math|Transform|MakeTransform "0.000000,-15.000000,10.000000" "90.000000,-90.000000,180.000000" "0.500000,0.500000,0.500000") :NewEnumerator2 (Math|Transform|MakeTransform "0.000000,-15.000000,2.000000" "0.000000,0.000000,-110.000000" "1.100000,1.100000,1.100000") :NewEnumerator3 (Math|Transform|MakeTransform "0.000000,180.000000,35.000000" "0.000000,0.000000,-100.000000" "1.200000,1.200000,1.200000") :NewEnumerator4 (Math|Transform|MakeTransform "0.000000,-18.000000,5.000000" "0, 0, 0" "15.000000,15.000000,15.000000") :NewEnumerator5 (Math|Transform|MakeTransform "0.000000,-20.000000,8.000000" "0.000000,0.000000,-100.000000" "0.200000,0.200000,0.200000") :NewEnumerator6 (Math|Transform|MakeTransform "0.000000,220.000000,0.000000" "0.000000,0.000000,-90.000000" "1.000000,1.000000,1.000000")) false false)
  (Variables|Default|SetMaskTransformRef (Utilities|Select :Index _output_get_3 :NewEnumerator0 (Math|Transform|MakeTransform "0.000000,-20.000000,15.000000" "90.000000,0.000000,-90.000000" "0.400000,0.400000,0.400000") :NewEnumerator1 (Math|Transform|MakeTransform "0.000000,-15.000000,10.000000" "90.000000,-90.000000,180.000000" "0.500000,0.500000,0.500000") :NewEnumerator2 (Math|Transform|MakeTransform "0.000000,-15.000000,2.000000" "0.000000,0.000000,-110.000000" "1.100000,1.100000,1.100000") :NewEnumerator3 (Math|Transform|MakeTransform "0.000000,180.000000,35.000000" "0.000000,0.000000,-100.000000" "1.200000,1.200000,1.200000") :NewEnumerator4 (Math|Transform|MakeTransform "0.000000,-18.000000,5.000000" "0, 0, 0" "15.000000,15.000000,15.000000") :NewEnumerator5 (Math|Transform|MakeTransform "0.000000,-20.000000,8.000000" "0.000000,0.000000,-100.000000" "0.200000,0.200000,0.200000") :NewEnumerator6 (Math|Transform|MakeTransform "0.000000,220.000000,0.000000" "0.000000,0.000000,-90.000000" "1.000000,1.000000,1.000000"))))

(event Custom|InitCharacter
  (bind _array (Utilities|Array|MakeArray "NewEnumerator0" "NewEnumerator1" "NewEnumerator2" "NewEnumerator3" "NewEnumerator4" "NewEnumerator5" "NewEnumerator6"))
  (bind _sm_mask (Variables|Default|GetSM_Mask))
  (bind _outitem (Utilities|Array|Random _array))
  (bind _output_get (Variables|Default|SetTopColor _outitem))
  (Rendering|Material|SetMaterial (Variables|Default|GetSK_Top) 0 (Utilities|Select :Index _output_get :NewEnumerator0 "/Game/Assets/Materials/MI_Cloth_Blue.MI_Cloth_Blue" :NewEnumerator1 "/Game/Assets/Materials/MI_Cloth_Red.MI_Cloth_Red" :NewEnumerator2 "/Game/Assets/Materials/MI_Cloth_Yellow.MI_Cloth_Yellow" :NewEnumerator3 "/Game/Assets/Materials/MI_Cloth_Green.MI_Cloth_Green" :NewEnumerator4 "/Game/Assets/Materials/MI_Cloth_Purple.MI_Cloth_Purple" :NewEnumerator5 "/Game/Assets/Materials/MI_Cloth_Pink.MI_Cloth_Pink" :NewEnumerator6 "/Game/Assets/Materials/MI_Cloth_Brown.MI_Cloth_Brown"))
  (bind _output_get_2 (Variables|Default|SetBottomColor _outitem))
  (Rendering|Material|SetMaterial (Variables|Default|GetSK_Bottom) 0 (Utilities|Select :Index _output_get_2 :NewEnumerator0 "/Game/Assets/Materials/MI_Cloth_Blue.MI_Cloth_Blue" :NewEnumerator1 "/Game/Assets/Materials/MI_Cloth_Red.MI_Cloth_Red" :NewEnumerator2 "/Game/Assets/Materials/MI_Cloth_Yellow.MI_Cloth_Yellow" :NewEnumerator3 "/Game/Assets/Materials/MI_Cloth_Green.MI_Cloth_Green" :NewEnumerator4 "/Game/Assets/Materials/MI_Cloth_Purple.MI_Cloth_Purple" :NewEnumerator5 "/Game/Assets/Materials/MI_Cloth_Pink.MI_Cloth_Pink" :NewEnumerator6 "/Game/Assets/Materials/MI_Cloth_Brown.MI_Cloth_Brown"))
  (bind _output_get_3 (Variables|Default|SetMask (.OutItem (Utilities|Array|Random (Utilities|Array|MakeArray "NewEnumerator0" "NewEnumerator1" "NewEnumerator2" "NewEnumerator3" "NewEnumerator4" "NewEnumerator5" "NewEnumerator6")))))
  (Components|StaticMesh|SetStaticMesh _sm_mask (Utilities|Select :Index _output_get_3 :NewEnumerator0 "/Game/Assets/Masks/Kitsune/7b6eb1ca7e6c_dark_fantasy__golde.7b6eb1ca7e6c_dark_fantasy__golde" :NewEnumerator1 "/Game/Assets/Masks/Blue/delft_blue_mask.delft_blue_mask" :NewEnumerator2 "/Game/Assets/Masks/Face/Mask.Mask" :NewEnumerator3 "/Game/Assets/Masks/Plague/Mask.Mask" :NewEnumerator4 "/Game/Assets/Masks/Hockey/джасан.джасан" :NewEnumerator5 "/Game/Assets/Masks/Venetian/venetian_mask_1.venetian_mask_1" :NewEnumerator6 "/Game/Assets/Masks/Wolf/wolfmask1.wolfmask1"))
  (Transformation|SetRelativeTransform _sm_mask (Utilities|Select :Index _output_get_3 :NewEnumerator0 (Math|Transform|MakeTransform "0.000000,-20.000000,15.000000" "90.000000,0.000000,-90.000000" "0.400000,0.400000,0.400000") :NewEnumerator1 (Math|Transform|MakeTransform "0.000000,-15.000000,10.000000" "90.000000,-90.000000,180.000000" "0.500000,0.500000,0.500000") :NewEnumerator2 (Math|Transform|MakeTransform "0.000000,-15.000000,2.000000" "0.000000,0.000000,-110.000000" "1.100000,1.100000,1.100000") :NewEnumerator3 (Math|Transform|MakeTransform "0.000000,180.000000,35.000000" "0.000000,0.000000,-100.000000" "1.200000,1.200000,1.200000") :NewEnumerator4 (Math|Transform|MakeTransform "0.000000,-18.000000,5.000000" "0, 0, 0" "15.000000,15.000000,15.000000") :NewEnumerator5 (Math|Transform|MakeTransform "0.000000,-20.000000,8.000000" "0.000000,0.000000,-100.000000" "0.200000,0.200000,0.200000") :NewEnumerator6 (Math|Transform|MakeTransform "0.000000,220.000000,0.000000" "0.000000,0.000000,-90.000000" "1.000000,1.000000,1.000000")) false false)
  (Variables|Default|SetMaskTransformRef (Utilities|Select :Index _output_get_3 :NewEnumerator0 (Math|Transform|MakeTransform "0.000000,-20.000000,15.000000" "90.000000,0.000000,-90.000000" "0.400000,0.400000,0.400000") :NewEnumerator1 (Math|Transform|MakeTransform "0.000000,-15.000000,10.000000" "90.000000,-90.000000,180.000000" "0.500000,0.500000,0.500000") :NewEnumerator2 (Math|Transform|MakeTransform "0.000000,-15.000000,2.000000" "0.000000,0.000000,-110.000000" "1.100000,1.100000,1.100000") :NewEnumerator3 (Math|Transform|MakeTransform "0.000000,180.000000,35.000000" "0.000000,0.000000,-100.000000" "1.200000,1.200000,1.200000") :NewEnumerator4 (Math|Transform|MakeTransform "0.000000,-18.000000,5.000000" "0, 0, 0" "15.000000,15.000000,15.000000") :NewEnumerator5 (Math|Transform|MakeTransform "0.000000,-20.000000,8.000000" "0.000000,0.000000,-100.000000" "0.200000,0.200000,0.200000") :NewEnumerator6 (Math|Transform|MakeTransform "0.000000,220.000000,0.000000" "0.000000,0.000000,-90.000000" "1.000000,1.000000,1.000000"))))

(event EventBeginPlay
  (CallFunction|InitCharacter)
  (CallFunction|AIMovement))

(event EventTick
  (params (DeltaSeconds :type Float%20%28single-precision%29)))

(fn ConstructionScript)