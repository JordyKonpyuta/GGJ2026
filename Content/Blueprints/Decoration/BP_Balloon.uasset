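; BP_Balloon is a decorative balloon actor that bobs up and down and appears in a random color.
; The construction script picks one of five balloon materials at random and applies it to both skeletal meshes.
; On BeginPlay, a timeline gets a random play rate and loops by restarting itself, driving the first mesh's relative Z position so balloons move out of sync.
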(event Custom|Move
  (bind _newtrack_0 (Timeline|Timeline PlayFromStart)
    (:Update
      (Transformation|SetRelativeLocation (Variables|Default|GetSkeletalMesh) (Math|Vector|MakeVector 0.0 0.0 (* _newtrack_0 5e+01)) false false))
    (:Finished
      (CallFunction|Move))))

(event EventBeginPlay
  (Components|Timeline|SetPlayRate (Variables|Default|GetTimeline) (+ (Math|Random|RandomFloat) 1.0))
  (CallFunction|Move))

(fn ConstructionScript
  (bind _output_get (Variables|Default|SetColor (Math|Random|RandomInteger 5)))
  (Rendering|Material|SetMaterial (Variables|Default|GetSkeletalMesh) 0 (Utilities|Select :Index _output_get :Option%200 "/Game/Assets/Balloon/balloon_blue_sh.balloon_blue_sh" :Option%201 "/Game/Assets/Balloon/balloon_red_sh.balloon_red_sh" :Option%202 "/Game/Assets/Balloon/balloon_skyblue_sh.balloon_skyblue_sh" :Option%203 "/Game/Assets/Balloon/balloon_white_sh.balloon_white_sh" :Option%204 "/Game/Assets/Balloon/balloon_yellow_sh.balloon_yellow_sh")))